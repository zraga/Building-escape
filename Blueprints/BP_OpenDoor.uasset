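; Door actor that swings open and closed in response to the OnOpen and OnClose events from OpenDoor.
; The DoorSwing timeline plays forward to open and reverses to close, adding its yaw curve to the rotation cached at BeginPlay.
; A Sound Timing event track on the timeline plays the Doorlock sound at the actor's location.
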(event OnClose(OpenDoor)
  (bind _opendoor (Timeline|DoorSwing Reverse)
    (:Update
      (Transformation|SetActorRotation (Math|Rotator|CombineRotators (Math|Rotator|MakeRotator 0.0 0.0 _opendoor) (Variables|Default|Getinitial%20rotation))))
    (:Sound%20timing
      (Audio|PlaySoundatLocation "/Game/Audio/door-lock.door-lock" (Transformation|GetActorLocation)))))

(event OnOpen(OpenDoor)
  (bind _opendoor (Timeline|DoorSwing Play)
    (:Update
      (Transformation|SetActorRotation (Math|Rotator|CombineRotators (Math|Rotator|MakeRotator 0.0 0.0 _opendoor) (Variables|Default|Getinitial%20rotation))))
    (:Sound%20timing
      (Audio|PlaySoundatLocation "/Game/Audio/door-lock.door-lock" (Transformation|GetActorLocation)))))

(event EventBeginPlay
  (Variables|Default|Setinitial%20rotation (Transformation|GetActorRotation)))

(fn ConstructionScript)